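; Trigger volume, apparently marking the beginning of a curve, that changes the ball's control state and applies curve damage when the ball enters it.
; On box overlap with PhysicsBallBP it runs BaseOverlap, inverts the ball's controls and turns off rolling mode.
; It then passes the DamageFromCurve value, read from the ball referenced by BallGameInstance, to ChangeHealth and resets that value to MinHealth.
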(event `self.ReceiveBeginPlay`
  (set `self.GameInstance` (cast `/Game/BluePrints/Savings/BallGameInstance` (`GameplayStatics.GetGameInstance`) :!pure true)))

(event `self.BoxTrigger.OnComponentBeginOverlap`
  (params (OverlappedComponent :type "PrimitiveComponent Object Reference") (OtherActor :type "Actor Object Reference") (OtherComp :type "PrimitiveComponent Object Reference") (OtherBodyIndex :type Integer) (bFromSweep :type Boolean) (SweepResult :type "HitResult Structure (by ref)"))
  (bind _ballpawn (`/Game/BluePrints/Savings/BallGameInstance.BallPawn` (`self.GameInstance`)))
  (bind _asphysics_ball_bp (cast `/Game/BluePrints/PhysicsBallBP` OtherActor))
  (bind _output_get (set `self.BallPawn` _asphysics_ball_bp))
  (`self.Base Overlap` _output_get)
  (set `/Game/BluePrints/PhysicsBallBP.IsControllInverted` true (`self.BallPawn`))
  (set `/Game/BluePrints/PhysicsBallBP.IsRollingMode` false (`self.Pawn`))
  (`/Game/BluePrints/PhysicsBallBP.ChangeHealth` (`self.BallPawn`) (`/Game/BluePrints/Savings/BallPawn.DamageFromCurve` (`/Game/BluePrints/Savings/BallGameInstance.BallPawn` (`self.GameInstance`))))
  (set `/Game/BluePrints/Savings/BallPawn.DamageFromCurve` (`/Game/BluePrints/Savings/BallPawn.MinHealth` _ballpawn) _ballpawn))

(fn `UserConstructionScript`
  (`parent.UserConstructionScript`))