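; Button actor that, when the physics ball overlaps it, lowers itself, moves a linked door vertically and starts a timed navigation widget.
; The widget receives the ball and win prize locations, with Tick updating ball position and elapsed count and triggering a countdown animation near the limit.
; Re-overlapping resets the running timer.
; A DestroyTimer event bound through BallGameInstance removes the widget and reverses both timelines.
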(event `self.ReceiveBeginPlay`
  (set `self.Pawn` (cast `/Game/BluePrints/PhysicsBallBP` (`GameplayStatics.GetPlayerPawn` 0) :!pure true))
  (set `self.GameInstance` (cast `/Game/BluePrints/Savings/BallGameInstance` (`GameplayStatics.GetGameInstance`) :!pure true))
  (set `self.InitialButtonLocation` (`SceneComponent.K2_GetComponentLocation` (`self.Button`)))
  (set `self.InitialDoorLocation` (`self.K2_GetActorLocation` (`self.Door`)))
  (add `/Game/BluePrints/Savings/BallGameInstance.DestroyTimer` (`self.GameInstance`) (delegate `DestroyTimer`)))

(event `DestroyTimer`
  (bind _widget (`self.Widget`))
  (bind (_initialbuttonlocation_x _initialbuttonlocation_y _initialbuttonlocation_z) (`KismetMathLibrary.BreakVector` (`self.InitialButtonLocation`)))
  (bind (_initialdoorlocation_x _initialdoorlocation_y _initialdoorlocation_z) (`KismetMathLibrary.BreakVector` (`self.InitialDoorLocation`)))
  (set `self.IsTimerAlreadyStarted` false)
  (`/Engine/EditorBlueprintResources/StandardMacros.IsValid` _widget
    (:`Is Valid`
      (`Widget.RemoveFromParent` _widget))
    (:`Is Not Valid`
      _))
  (set `self.Count` 0.0)
  (set `self.Widget` null)
  (`|ExecutionSequence`
    (:`then_0`
      (bind (_direction _zvalue) (`Timeline|ButtonDescent` :!via `Reverse` :!label _label)
        (:`Update`
          (`SceneComponent.K2_SetWorldLocation` (`self.Button`) (`KismetMathLibrary.MakeVector` _initialbuttonlocation_x _initialbuttonlocation_y (- _initialbuttonlocation_z _zvalue)) false false))))
    (:`then_1`
      (bind (_direction_2 _door) (`Timeline|DoorDescent` :!via `Reverse` :!label _label_2)
        (:`Update`
          (`self.K2_SetActorLocation` (`self.Door`) (`KismetMathLibrary.MakeVector` _initialdoorlocation_x _initialdoorlocation_y (+ _initialdoorlocation_z _door)) false false))))))

(event `self.Sphere.OnComponentBeginOverlap`
  (params (OverlappedComponent :type "PrimitiveComponent Object Reference") (OtherActor :type "Actor Object Reference") (OtherComp :type "PrimitiveComponent Object Reference") (OtherBodyIndex :type Integer) (bFromSweep :type Boolean) (SweepResult :type "HitResult Structure (by ref)"))
  (cast `/Game/BluePrints/PhysicsBallBP` OtherActor)
  (`|ExecutionSequence`
    (:`then_0`
      (if (== (`self.IsTimerAlreadyStarted`) false)
        (goto _label :!via `PlayFromStart`)))
    (:`then_1`
      (if (== (`self.IsTimerAlreadyStarted`) false)
        (goto _label_2 :!via `PlayFromStart`)))
    (:`then_2`
      (`self.SetTimer`))))

(event `SetTimer`
  (if (== (`self.IsTimerAlreadyStarted`) false)
    (bind _returnvalue (`|CreateWidget` "/Game/Widgets/Navigation.Navigation_C"))
    (set `self.Widget` _returnvalue)
    (set `/Game/Widgets/Navigation.PawnLocation` (`SceneComponent.K2_GetComponentLocation` (`/Game/BluePrints/PhysicsBallBP.Ball` (`self.Pawn`))) (`self.Widget`))
    (set `/Game/Widgets/Navigation.WinPrizeLocation` (`SceneComponent.K2_GetComponentLocation` (`/Game/BluePrints/BP_WinPickUp.Niagara` (`self.WinPrize`))) (`self.Widget`))
    (set `/Game/Widgets/Navigation.TimerInitialValue` (`self.TimerInitialValue`) (`self.Widget`))
    (`UserWidget.AddToViewport` (`self.Widget`) 0)
    (set `self.IsTimerAlreadyStarted` true)
    (else
      (`self.ResetTimer`))))

(event `self.ReceiveTick`
  (params (DeltaSeconds :type "Float (single-precision)"))
  (if (== (`self.IsTimerAlreadyStarted`) true)
    (`self.ManageTimer` DeltaSeconds)
    (set `/Game/Widgets/Navigation.PawnLocation` (`SceneComponent.K2_GetComponentLocation` (`/Game/BluePrints/PhysicsBallBP.Ball` (`self.Pawn`))) (`self.Widget`))))

(fn `ManageTimer`
  (params (DeltaSeconds :type "Float (double-precision)"))
  (locals (MinTreshholdStartAnimation :type "Float (double-precision)" :default 3.0) (MinTreshholdCount :type "Float (double-precision)" :default 0.2))
  (bind _widget (`self.Widget`))
  (`|ExecutionSequence`
    (:`then_0`
      (set `self.Count` (+ (`self.Count`) DeltaSeconds)))
    (:`then_1`
      (if (<= (mod (`self.Count`) 1.0) (`local.MinTreshholdCount`))
        (set `/Game/Widgets/Navigation.Count` (`KismetMathLibrary.Conv_IntToDouble` (`KismetMathLibrary.FTrunc` (`self.Count`))) (`self.Widget`))))
    (:`then_2`
      (if (<= (- (`self.TimerInitialValue`) (`self.Count`)) (`local.MinTreshholdStartAnimation`))
        (if (and (== (`KismetSystemLibrary.IsValid` (`self.Widget`)) true) (!= (`/Game/Widgets/Navigation.IsAnimationStarted` (`self.Widget`)) true))
          (`UserWidget.PlayAnimation` _widget (`/Game/Widgets/Navigation.CountdownAnimation` _widget) 0.0 1 "Forward" 1.0 true)
          (set `/Game/Widgets/Navigation.IsAnimationStarted` true (`self.Widget`)))))))

(fn `ResetTimer`
  (bind _widget (`self.Widget`))
  (bind _widget_2 (`self.Widget`))
  (set `self.Count` (`self.CountInitialValue`))
  (`/Engine/EditorBlueprintResources/StandardMacros.IsValid` (`self.Widget`)
    (:`Is Valid`
      (set `/Game/Widgets/Navigation.IsAnimationStarted` false (`self.Widget`))
      (if (`UserWidget.IsAnimationPlaying` _widget_2 (`/Game/Widgets/Navigation.CountdownAnimation` _widget_2))
        (`UserWidget.StopAnimation` _widget (`/Game/Widgets/Navigation.CountdownAnimation` _widget))))))

(fn `UserConstructionScript`)