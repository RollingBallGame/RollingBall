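; BallGameInstance is the game instance for a rolling-ball game, holding score, checkpoint state and background music across levels.
; PrepareCurrentLevel finds the BP_SaveOptions actor whose checkpoint tag matches the stored teleportation tag, then applies its rolling, inverted-control and camera-volume settings.
; Helpers reset state for the next level and set game-over flags.
; A BackgroundSong object tracks played time via real-time timestamps, resuming the track with looped wraparound.
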(event `self.ReceiveInit`
  (bind _returnvalue (`|GenericCreateObject` "/Game/BluePrints/Savings/BallPawn.BallPawn_C" self))
  (set `self.BallPawn` _returnvalue))

(fn `CalculateSongStartTIme`
  (bind _bgsong (`self.BGSong`))
  (bind _duration (`/Game/BluePrints/Savings/BackgroundSong.Duration` _bgsong))
  (set `/Game/BluePrints/Savings/BackgroundSong.PlayedTime` (- (`/Game/BluePrints/Savings/BackgroundSong.PlayedTime` (`self.BGSong`)) (* (`KismetMathLibrary.FTrunc` (/ (`/Game/BluePrints/Savings/BackgroundSong.PlayedTime` _bgsong) _duration)) _duration)) (`self.BGSong`)))

(fn `IncreaseScore`
  (params (ScoreAddition :type Integer))
  (set `self.Score` (+ ScoreAddition (`self.Score`))))

(fn `PreGameFinishStuff`
  (params (ShouldWaitTimeOfHealthDecrease :type Boolean) (ShouldPlayGameSound :type Boolean))
  (set `self.ShouldWaitTimeOfHealthDecrease` ShouldWaitTimeOfHealthDecrease)
  (set `self.ShouldPlayGameOverSound` ShouldPlayGameSound))

(fn `PreparationForNextLevel`
  (`self.ResetTeleportationTag`)
  (set `self.IsStartOfTheGame` true)
  (set `self.IsLoadFromStart` true))

(fn `PrepareCurrentLevel`
  (set `self.Pawn` (cast `/Game/BluePrints/PhysicsBallBP` (`GameplayStatics.GetPlayerPawn` 0) :!pure true))
  (bind _outactors (`GameplayStatics.GetAllActorsOfClass` "/Game/BluePrints/Savings/BP_SaveOptions.BP_SaveOptions_C"))
  (for _array_element _outactors
    (if (== (`/Game/BluePrints/Savings/BP_SaveOptions.CheckpointTag` _array_element) (`self.TeleportationTag`))
      (set `self.CurrentSaveOption` _array_element)
      (set `/Game/BluePrints/PhysicsBallBP.IsRollingMode` (`/Game/BluePrints/Savings/BP_SaveOptions.IsRollingMode` (`self.CurrentSaveOption`)) (`self.Pawn`))
      (set `/Game/BluePrints/PhysicsBallBP.IsControllInverted` (`/Game/BluePrints/Savings/BP_SaveOptions.IsControllInverted` (`self.CurrentSaveOption`)) (`self.Pawn`))
      (set `self.IsCameraVolumeUsing` (`/Game/BluePrints/Savings/BP_SaveOptions.IsCameraVolumeUsing` (`self.CurrentSaveOption`)))
      (if (`/Game/BluePrints/Savings/BP_SaveOptions.IsCameraVolumeUsing` (`self.CurrentSaveOption`))
        (set `self.CurrentCameraVolume` (`/Game/BluePrints/Savings/BP_SaveOptions.CurrentCameraVolume` (`self.CurrentSaveOption`)))
        (set `self.IsCameraRotatable` (`/Game/BluePrints/Savings/BP_SaveOptions.IsCameraRotatable` (`self.CurrentSaveOption`)))))))

(fn `ResetTeleportationTag`
  (set `self.TeleportationTag` (`self.TeleportationTagDefault`)))

(fn `StartBGSong`
  (bind _bgsong (`self.BGSong`))
  (`/Engine/EditorBlueprintResources/StandardMacros.IsValid` (`self.BGSong`)
    (:`Is Valid`
      (if (> (`/Game/BluePrints/Savings/BackgroundSong.PlayedTime` _bgsong) (`/Game/BluePrints/Savings/BackgroundSong.Duration` _bgsong))
        (`self.CalculateSongStartTIme`))
      (bind _returnvalue (`GameplayStatics.SpawnSound2D` "/Game/Sound/Harry-Styles-As-It-Was.Harry-Styles-As-It-Was" 1.0 1.0 (`/Game/BluePrints/Savings/BackgroundSong.PlayedTime` (`self.BGSong`)) null))
      (set `/Game/BluePrints/Savings/BackgroundSong.Song` _returnvalue (`self.BGSong`)))
    (:`Is Not Valid`
      (bind _returnvalue_2 (`|GenericCreateObject` "/Game/BluePrints/Savings/BackgroundSong.BackgroundSong_C" self))
      (set `self.BGSong` _returnvalue_2)
      (bind _returnvalue_3 (`GameplayStatics.SpawnSound2D` "/Game/Sound/Harry-Styles-As-It-Was.Harry-Styles-As-It-Was" 1.0 1.0 0.0 null))
      (set `/Game/BluePrints/Savings/BackgroundSong.Song` _returnvalue_3 (`self.BGSong`))
      (set `/Game/BluePrints/Savings/BackgroundSong.TimeStart` (`GameplayStatics.GetRealTimeSeconds`) (`self.BGSong`))
      (set `/Game/BluePrints/Savings/BackgroundSong.Duration` (`SoundBase.Duration` (`AudioComponent.Sound` _returnvalue_3)) (`self.BGSong`)))))

(fn `UpdateBGSongPlayTime`
  (bind _bgsong (`self.BGSong`))
  (bind _output_get (set `/Game/BluePrints/Savings/BackgroundSong.TimeEnd` (`GameplayStatics.GetRealTimeSeconds`) (`self.BGSong`)))
  (set `/Game/BluePrints/Savings/BackgroundSong.PlayedTime` (+ (- _output_get (`/Game/BluePrints/Savings/BackgroundSong.TimeStart` (`self.BGSong`))) (`/Game/BluePrints/Savings/BackgroundSong.PlayedTime` _bgsong)) _bgsong))