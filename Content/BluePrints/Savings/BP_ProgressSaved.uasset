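; BP_ProgressSaved is a checkpoint trigger that records progress when the player's physics ball overlaps its box.
; On a new tag, it stores its teleportation tag in BallGameInstance and clears the load-from-start flag.
; It then spawns a BP_WidgetAnimation at the default widget location, calls SaveProgress on it, and clears the game instance's widget reference.
; Re-entering the checkpoint whose tag is already stored does nothing.
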(event `self.Box.OnComponentBeginOverlap`
  (params (OverlappedComponent :type "PrimitiveComponent Object Reference") (OtherActor :type "Actor Object Reference") (OtherComp :type "PrimitiveComponent Object Reference") (OtherBodyIndex :type Integer) (bFromSweep :type Boolean) (SweepResult :type "HitResult Structure (by ref)"))
  (cast `/Game/BluePrints/PhysicsBallBP` OtherActor)
  (set `self.GameInstance` (cast `/Game/BluePrints/Savings/BallGameInstance` (`GameplayStatics.GetGameInstance`) :!pure true))
  (if (!= (`/Game/BluePrints/Savings/BallGameInstance.TeleportationTag` (`self.GameInstance`)) (`self.CurrentTeleportationTag`))
    (set `/Game/BluePrints/Savings/BallGameInstance.TeleportationTag` (`self.CurrentTeleportationTag`) (`self.GameInstance`))
    (set `/Game/BluePrints/Savings/BallGameInstance.IsLoadFromStart` false (`self.GameInstance`))
    (bind _returnvalue (`|SpawnActorFromClass` "/Game/BluePrints/BP_WidgetAnimation.BP_WidgetAnimation_C" (`/Game/BluePrints/Savings/BallGameInstance.DefaultWidgetLocation` (`self.GameInstance`)) "Undefined" "OverrideRootScale" null null))
    (bind _output_get (set `/Game/BluePrints/Savings/BallGameInstance.Widget` _returnvalue (`self.GameInstance`)))
    (`/Game/BluePrints/BP_WidgetAnimation.SaveProgress` _output_get)
    (set `/Game/BluePrints/Savings/BallGameInstance.Widget` null (`self.GameInstance`))))

(fn `UserConstructionScript`)