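; HUD for the rolling-ball game that creates startup widgets, starts background music and handles game over and win.
; It binds to GameInstance events; game over can wait for health decrease and resets pawn health, while a win stops the music.
; Both feed LevelEnd, which clears widgets, pauses, switches to UI input, shows the result widget and optionally plays its sound.
; LevelEnd also applies a dynamic BlackWhite post-process material to the active volume or pawn camera.
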(event `GameOver`
  (if (== (`/Game/BluePrints/Savings/BallGameInstance.ShouldWaitTimeOfHealthDecrease` (`self.GameInstance`)) true)
    (`KismetSystemLibrary.Delay` (`self.TimeOfHealthDecrease`)))
  (`self.Level End` "/Game/Widgets/GameOver.GameOver_C" "/Game/Sound/GameOver.GameOver")
  (`/Game/BluePrints/PhysicsBallBP.ResetHealth` (`self.Pawn`)))

(event `self.ReceiveBeginPlay`
  (bind _output_get (set `self.GameInstance` (cast `/Game/BluePrints/Savings/BallGameInstance` (`GameplayStatics.GetGameInstance`) :!pure true)))
  (`/Game/BluePrints/Savings/BallGameInstance.StartBGSong` _output_get)
  (for _array_element (`self.WidgetsToInit`)
    (`self.InitWidget` _array_element)
    (set `self.Pawn` (cast `/Game/BluePrints/PhysicsBallBP` (`GameplayStatics.GetPlayerPawn` 0) :!pure true))
    (add `/Game/BluePrints/Savings/BallGameInstance.GameOver` (`self.GameInstance`) (delegate `GameOver`))
    (add `/Game/BluePrints/Savings/BallGameInstance.GameWin` (`self.GameInstance`) (delegate `GamWIn`))))

(event `GamWIn`
  (`AudioComponent.Stop` (`/Game/BluePrints/Savings/BackgroundSong.Song` (`/Game/BluePrints/Savings/BallGameInstance.BGSong` (`self.GameInstance`))))
  (`self.Level End` "/Game/Widgets/GameWIn.GameWIn_C" "/Game/Sound/GameWin.GameWin"))

(fn `ChangeCameraPostProcess`
  (bind _returnvalue (`KismetMaterialLibrary.CreateDynamicMaterialInstance` "/Game/Materials/BlackWhite.BlackWhite"))
  (bind _output_get (set `self.DynamicMaterial` _returnvalue))
  (bind _currentcamera (`self.GetCurrentCamera`))
  (set `CameraComponent.PostProcessSettings` (make `PostProcessSettings` :`WeightedBlendables` (make `WeightedBlendables` (`|MakeArray` (make `WeightedBlendable` 1.0 _output_get)))) _currentcamera)
  (`MaterialInstanceDynamic.SetScalarParameterValue` (`self.DynamicMaterial`) "Intensity" 0.0))

(fn `GetCurrentCamera`
  (returns (CurrentCamera :type "CameraComponent Object Reference"))
  (locals (Camera :type "CameraComponent Object Reference"))
  (if (`/Game/BluePrints/Savings/BallGameInstance.IsCameraVolumeUsing` (`self.GameInstance`))
    (set `local.Camera` (`/Game/BluePrints/BP_CameraVolume.Camera` (`/Game/BluePrints/Savings/BallGameInstance.CurrentCameraVolume` (`self.GameInstance`))))
    (else
      (set `local.Camera` (`/Game/BluePrints/PhysicsBallBP.Camera` (`self.Pawn`)))))
  (return (`local.Camera`)))

(fn `InitWidget`
  (params (Class :type "UserWidget Class Reference"))
  (bind _returnvalue (`|CreateWidget` Class))
  (`UserWidget.AddToViewport` _returnvalue 0))

(fn `Level End`
  (params (Widget :type "UserWidget Class Reference") (Sound :type "SoundBase Object Reference"))
  (locals (UserWidget :type "UserWidget Class Reference") (FinalSound :type "SoundBase Object Reference"))
  (bind _returnvalue (`GameplayStatics.GetPlayerController` 0))
  (bind _jumpsound (`/Game/BluePrints/PhysicsBallBP.JumpSound` (`self.Pawn`)))
  (set `local.UserWidget` Widget)
  (set `local.FinalSound` Sound)
  (`/Engine/EditorBlueprintResources/StandardMacros.IsValid` (`/Game/BluePrints/Savings/BallGameInstance.Widget` (`self.GameInstance`))
    (:`Is Valid`
      (`self.K2_DestroyActor` (`/Game/BluePrints/Savings/BallGameInstance.Widget` (`self.GameInstance`)))
      (set `/Game/BluePrints/Savings/BallGameInstance.Widget` null (`self.GameInstance`)))
    (:`Is Not Valid`
      _))
  (`WidgetLayoutLibrary.RemoveAllWidgets`)
  (`GameplayStatics.SetGamePaused` true)
  (set `PlayerController.bShowMouseCursor` true _returnvalue)
  (`WidgetBlueprintLibrary.SetInputMode_UIOnlyEx` _returnvalue null)
  (`self.ChangeCameraPostProcess`)
  (bind _returnvalue_2 (`|CreateWidget` (`local.UserWidget`)))
  (`UserWidget.AddToViewport` _returnvalue_2 0)
  (if (`KismetSystemLibrary.IsValid` _jumpsound)
    (`AudioComponent.Stop` _jumpsound)
    (set `/Game/BluePrints/PhysicsBallBP.JumpSound` null (`self.Pawn`)))
  (if (== (`/Game/BluePrints/Savings/BallGameInstance.ShouldPlayGameOverSound` (`self.GameInstance`)) true)
    (`GameplayStatics.PlaySound2D` (`local.FinalSound`) 1.0 1.0 0.0 null null)))

(fn `UserConstructionScript`)