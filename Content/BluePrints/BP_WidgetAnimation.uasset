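; Short-lived actor that shows animated overlay widgets for level start, checkpoint load and saved progress.
; ChooseWidget reads BallGameInstance to pick the level intro or, when a non-default teleportation tag is set, the checkpoint widget.
; EntryWidget creates and plays that widget, matching on class display name, while SaveProgress builds its own.
; Each path waits for the animation's length, then destroys the actor, whose Destroyed event removes the widget.
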(event `ChooseWidget`
  (bind _gameinstance (`self.GameInstance`))
  (set `self.GameInstance` (cast `/Game/BluePrints/Savings/BallGameInstance` (`GameplayStatics.GetGameInstance`) :!pure true))
  (if (== (`/Game/BluePrints/Savings/BallGameInstance.IsStartOfTheGame` (`self.GameInstance`)) true)
    (`self.EntryWidget` "/Game/Widgets/Level.Level_C")
    (`KismetSystemLibrary.Delay` (`self.TimeOfAnimation`))
    (set `/Game/BluePrints/Savings/BallGameInstance.IsStartOfTheGame` false (`self.GameInstance`))
    (`self.K2_DestroyActor` :!label _label)
    (elif (!= (`/Game/BluePrints/Savings/BallGameInstance.TeleportationTag` _gameinstance) (`/Game/BluePrints/Savings/BallGameInstance.TeleportationTagDefault` _gameinstance))
      (`self.EntryWidget` "/Game/Widgets/LoadFromCheckpoint.LoadFromCheckpoint_C")
      (`KismetSystemLibrary.Delay` (`self.TimeOfAnimation`))
      (goto _label))))

(event `SaveProgress`
  (bind _widget (`self.Widget`))
  (bind _progressavedanimation (`/Game/Widgets/SaveProgress.ProgresSavedAnimation` (cast `/Game/Widgets/SaveProgress` _widget :!pure true)))
  (bind _returnvalue (`|CreateWidget` "/Game/Widgets/SaveProgress.SaveProgress_C"))
  (bind _output_get (set `self.Widget` _returnvalue))
  (`UserWidget.AddToViewport` _output_get 0)
  (set `self.TimeOfAnimation` (`WidgetAnimation.GetEndTime` _progressavedanimation))
  (`UserWidget.PlayAnimation` _widget _progressavedanimation 0.0 1 "Forward" 1.0 false)
  (`KismetSystemLibrary.Delay` (`self.TimeOfAnimation`))
  (`self.K2_DestroyActor`))

(event `self.ReceiveDestroyed`
  (`Widget.RemoveFromParent` (`self.Widget`)))

(fn `EntryWidget`
  (params (UserWidget :type "UserWidget Class Reference"))
  (bind _widget (`self.Widget`))
  (`/Engine/EditorBlueprintResources/StandardMacros.IsValid` _widget
    (:`Is Valid`
      (`Widget.RemoveFromParent` _widget))
    (:`Is Not Valid`
      _))
  (bind _returnvalue (`|CreateWidget` UserWidget))
  (bind _output_get (set `self.Widget` _returnvalue))
  (`UserWidget.AddToViewport` _output_get 0)
  (switch `string` (`KismetSystemLibrary.GetClassDisplayName` UserWidget)
    (:`Level_C`
      (bind _aslevel (cast `/Game/Widgets/Level` (`self.Widget`)))
      (bind _startuplevel (`/Game/Widgets/Level.StartupLevel` _aslevel))
      (set `self.TimeOfAnimation` (`WidgetAnimation.GetEndTime` _startuplevel))
      (`UserWidget.PlayAnimation` _aslevel _startuplevel 0.0 1 "Forward" 1.0 false))
    (:`LoadFromCheckpoint_C`
      (bind _asload_from_checkpoint (cast `/Game/Widgets/LoadFromCheckpoint` (`self.Widget`)))
      (bind _loadfromcheckpoint (`/Game/Widgets/LoadFromCheckpoint.LoadFromCheckpoint` _asload_from_checkpoint))
      (set `self.TimeOfAnimation` (`WidgetAnimation.GetEndTime` _loadfromcheckpoint))
      (`UserWidget.PlayAnimation` _asload_from_checkpoint _loadfromcheckpoint 0.0 1 "Forward" 1.0 false))))

(fn `UserConstructionScript`)