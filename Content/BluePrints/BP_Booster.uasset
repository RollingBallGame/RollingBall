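; BP_Booster is a booster that launches the physics ball when it enters the sphere trigger.
; On overlap it applies a velocity-change impulse along the static mesh's up vector, scaled by BoosterScalingFactor, so mesh orientation sets the launch direction.
; It also plays a 2D in-the-air sound, stores it in the ball's JumpSound, and turns on the ball's Niagara effect.
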(event `self.Sphere.OnComponentBeginOverlap`
  (params (OverlappedComponent :type "PrimitiveComponent Object Reference") (OtherActor :type "Actor Object Reference") (OtherComp :type "PrimitiveComponent Object Reference") (OtherBodyIndex :type Integer) (bFromSweep :type Boolean) (SweepResult :type "HitResult Structure (by ref)"))
  (bind _asphysics_ball_bp (cast `/Game/BluePrints/PhysicsBallBP` OtherActor))
  (set `self.Pawn` _asphysics_ball_bp)
  (bind _returnvalue (`GameplayStatics.SpawnSound2D` "/Game/Sound/BallInTheAir_Cue.BallInTheAir_Cue" 1.0 1.0 0.0 null))
  (set `/Game/BluePrints/PhysicsBallBP.JumpSound` _returnvalue (`self.Pawn`))
  (`PrimitiveComponent.AddImpulse` (`/Game/BluePrints/PhysicsBallBP.Ball` (`self.Pawn`)) (* (`SceneComponent.GetUpVector` (`self.StaticMesh`)) (`self.BoosterScalingFactor`)) "None" true)
  (`/Game/BluePrints/PhysicsBallBP.TurnOnNiagara` (`self.Pawn`)))

(fn `UserConstructionScript`)