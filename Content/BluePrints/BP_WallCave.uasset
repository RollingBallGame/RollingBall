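; BP_WallCave is a cave wall actor that halts the physics ball on contact and reacts to a weather change.
; Overlapping BoxWallDoor calls StopMovement, which cancels the ball's linear velocity with an opposite velocity-change impulse.
; On BeginPlay it binds ChangeMaterial to BallGameInstance's change-to-cloud weather event, which swaps MiddleDoor to a red lamp material after a delay.
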(event `self.BoxWallDoor.OnComponentBeginOverlap`
  (params (OverlappedComponent :type "PrimitiveComponent Object Reference") (OtherActor :type "Actor Object Reference") (OtherComp :type "PrimitiveComponent Object Reference") (OtherBodyIndex :type Integer) (bFromSweep :type Boolean) (SweepResult :type "HitResult Structure (by ref)"))
  (bind _asphysics_ball_bp (cast `/Game/BluePrints/PhysicsBallBP` OtherActor))
  (set `self.Pawn` _asphysics_ball_bp)
  (`self.StopMovement`))

(event `self.ReceiveBeginPlay`
  (set `self.Pawn` (cast `/Game/BluePrints/PhysicsBallBP` (`GameplayStatics.GetPlayerPawn` 0) :!pure true))
  (add `/Game/BluePrints/Savings/BallGameInstance.ChangeWeatherToCloud` (cast `/Game/BluePrints/Savings/BallGameInstance` (`GameplayStatics.GetGameInstance`) :!pure true) (delegate `ChangeMaterial`)))

(event `ChangeMaterial`
  (`KismetSystemLibrary.Delay` (`self.Duration`))
  (`PrimitiveComponent.SetMaterial` (`self.MiddleDoor`) 0 "/Game/AutomotiveMaterials/Materials/Exterior/Lights/MI_Lamp_Red1.MI_Lamp_Red1"))

(fn `StopMovement`
  (bind _returnvalue (`PrimitiveComponent.GetPhysicsLinearVelocity` (`/Game/BluePrints/PhysicsBallBP.Ball` (`self.Pawn`)) "None"))
  (`PrimitiveComponent.AddImpulse` (`/Game/BluePrints/PhysicsBallBP.Ball` (`self.Pawn`)) (* _returnvalue -1) "None" true))

(fn `UserConstructionScript`)