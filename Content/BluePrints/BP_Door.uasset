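; BP_Door is a hazard that destroys the player's physics ball and triggers game over on contact.
; When a PhysicsBallBP overlaps its Box, it plays the Ball_Explosion sound, hides the ball mesh and reveals the pawn's own Explosion component at the ball's location.
; It then has BallGameInstance run PreGameFinishStuff, with the health-decrease wait and game sound disabled, before calling CallGameOver.
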(event `self.Box.OnComponentBeginOverlap`
  (params (OverlappedComponent :type "PrimitiveComponent Object Reference") (OtherActor :type "Actor Object Reference") (OtherComp :type "PrimitiveComponent Object Reference") (OtherBodyIndex :type Integer) (bFromSweep :type Boolean) (SweepResult :type "HitResult Structure (by ref)"))
  (bind _asphysics_ball_bp (cast `/Game/BluePrints/PhysicsBallBP` OtherActor))
  (set `self.Pawn` _asphysics_ball_bp)
  (set `self.GameInstance` (cast `/Game/BluePrints/Savings/BallGameInstance` (`GameplayStatics.GetGameInstance`) :!pure true))
  (`GameplayStatics.PlaySound2D` "/Game/Sound/Ball_Explosion.Ball_Explosion" 1.0 1.0 0.0 null null)
  (set `self.BallLocation` (`SceneComponent.K2_GetComponentLocation` (`/Game/BluePrints/PhysicsBallBP.Ball` (`self.Pawn`))))
  (`SceneComponent.SetVisibility` (`/Game/BluePrints/PhysicsBallBP.Ball` (`self.Pawn`)) false false)
  (`SceneComponent.K2_SetWorldLocation` (`/Game/BluePrints/PhysicsBallBP.Explosion` (`self.Pawn`)) (`self.BallLocation`) false false)
  (`SceneComponent.SetHiddenInGame` (`/Game/BluePrints/PhysicsBallBP.Explosion` (`self.Pawn`)) false false)
  (`/Game/BluePrints/Savings/BallGameInstance.PreGameFinishStuff` (`self.GameInstance`) false false)
  (`/Game/BluePrints/Savings/BallGameInstance.GameOver` (`self.GameInstance`)))

(fn `UserConstructionScript`)