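; BP_BoosterArea is a speed boost zone that launches the physics ball when it enters the area.
; On begin play it disables collision on its static mesh, leaving the Box component to detect overlaps.
; An overlapping PhysicsBallBP triggers a 2D speed sound, turns on its Niagara effect and gets a velocity-change impulse along fixed world +X, independent of the booster's rotation.
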(event `self.ReceiveBeginPlay`
  (`PrimitiveComponent.SetCollisionEnabled` (`self.StaticMesh`) "NoCollision"))

(event `self.Box.OnComponentBeginOverlap`
  (params (OverlappedComponent :type "PrimitiveComponent Object Reference") (OtherActor :type "Actor Object Reference") (OtherComp :type "PrimitiveComponent Object Reference") (OtherBodyIndex :type Integer) (bFromSweep :type Boolean) (SweepResult :type "HitResult Structure (by ref)"))
  (bind _asphysics_ball_bp (cast `/Game/BluePrints/PhysicsBallBP` OtherActor))
  (set `self.Pawn` _asphysics_ball_bp)
  (`GameplayStatics.PlaySound2D` "/Game/Sound/Speed.Speed" 1.0 1.0 0.0 null null)
  (`/Game/BluePrints/PhysicsBallBP.TurnOnNiagara` (`self.Pawn`))
  (`PrimitiveComponent.AddImpulse` (`/Game/BluePrints/PhysicsBallBP.Ball` (`self.Pawn`)) (2000.0 0.0 0.0) "None" true))

(fn `UserConstructionScript`)