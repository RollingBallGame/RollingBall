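; BP_CameraVolume is a trigger volume that switches the player's view to itself when the physics ball enters its box.
; On overlap it registers itself as the current camera volume in BallGameInstance and passes on whether the camera is rotatable.
; It then blends the first player controller's view target to this actor using configurable blend time and function.
; An optional flag also makes the game instance change the weather to cloud.
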(event `self.ReceiveBeginPlay`
  (`parent.ReceiveBeginPlay`))

(event `self.Box.OnComponentBeginOverlap`
  (params (OverlappedComponent :type "PrimitiveComponent Object Reference") (OtherActor :type "Actor Object Reference") (OtherComp :type "PrimitiveComponent Object Reference") (OtherBodyIndex :type Integer) (bFromSweep :type Boolean) (SweepResult :type "HitResult Structure (by ref)"))
  (bind _asphysics_ball_bp (cast `/Game/BluePrints/PhysicsBallBP` OtherActor))
  (set `self.Pawn` _asphysics_ball_bp)
  (set `self.GameInstance` (cast `/Game/BluePrints/Savings/BallGameInstance` (`GameplayStatics.GetGameInstance`) :!pure true))
  (set `/Game/BluePrints/Savings/BallGameInstance.CurrentCameraVolume` self (`self.GameInstance`))
  (set `/Game/BluePrints/Savings/BallGameInstance.IsCameraRotatable` (`self.IsCameraRotatable`) (`self.GameInstance`))
  (`PlayerController.SetViewTargetWithBlend` (`GameplayStatics.GetPlayerController` 0) self (`self.Blend Time`) (`self.Blend Func`) 0.0 false)
  (if (== (`self.ChangeWeather`) true)
    (`/Game/BluePrints/Savings/BallGameInstance.ChangeWeatherToCloud` (`self.GameInstance`))))

(fn `UserConstructionScript`
  (`parent.UserConstructionScript`))