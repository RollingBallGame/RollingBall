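; BP_WinPickUp is a level-completion pickup that triggers a win when anything overlaps its capsule.
; The overlap notifies BallGameInstance of the level win, hides the Niagara effect, optionally delays, then has the instance prepare for the next level and save background song play time.
; On the last level it runs pre-finish steps, resets the teleportation tag and calls game win; otherwise it opens the next level by name.
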(event `self.Capsule.OnComponentBeginOverlap`
  (params (OverlappedComponent :type "PrimitiveComponent Object Reference") (OtherActor :type "Actor Object Reference") (OtherComp :type "PrimitiveComponent Object Reference") (OtherBodyIndex :type Integer) (bFromSweep :type Boolean) (SweepResult :type "HitResult Structure (by ref)"))
  (set `self.GameInstance` (cast `/Game/BluePrints/Savings/BallGameInstance` (`GameplayStatics.GetGameInstance`) :!pure true))
  (`/Game/BluePrints/Savings/BallGameInstance.LevelWin` (`self.GameInstance`))
  (`SceneComponent.SetVisibility` (`self.Niagara`) false false)
  (if (`self.ShouldUseDelay`)
    (`KismetSystemLibrary.Delay` (`self.DelayDuration`)))
  (`/Game/BluePrints/Savings/BallGameInstance.PreparationForNextLevel` (`self.GameInstance`))
  (`/Game/BluePrints/Savings/BallGameInstance.UpdateBGSongPlayTime` (`self.GameInstance`))
  (if (`self.IsLastLevel`)
    (`/Game/BluePrints/Savings/BallGameInstance.PreGameFinishStuff` (`self.GameInstance`) false true)
    (`/Game/BluePrints/Savings/BallGameInstance.ResetTeleportationTag` (`self.GameInstance`))
    (`/Game/BluePrints/Savings/BallGameInstance.GameWin` (`self.GameInstance`))
    (else
      (`GameplayStatics.OpenLevel` (`self.NextLevel`) false))))

(fn `UserConstructionScript`)