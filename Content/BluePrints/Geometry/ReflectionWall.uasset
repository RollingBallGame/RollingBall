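; ReflectionWall is a wall that bounces the physics ball in a preset direction and plays a bounce sound.
; When a PhysicsBallBP overlaps its Box, it reads the ball's velocity and picks the right or left reflection impulse from the ball's rolling-direction flag.
; It cancels the current motion with a negated-velocity impulse, then adds the chosen impulse, both as velocity changes, so the rebound ignores incoming angle and mass.
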(event `self.Box.OnComponentBeginOverlap`
  (params (OverlappedComponent :type "PrimitiveComponent Object Reference") (OtherActor :type "Actor Object Reference") (OtherComp :type "PrimitiveComponent Object Reference") (OtherBodyIndex :type Integer) (bFromSweep :type Boolean) (SweepResult :type "HitResult Structure (by ref)"))
  (bind _asphysics_ball_bp (cast `/Game/BluePrints/PhysicsBallBP` OtherActor))
  (set `self.Actor` _asphysics_ball_bp)
  (`self.GetReflectionImpulse`)
  (`self.ReboundFromSurface`)
  (`GameplayStatics.PlaySound2D` "/Game/Sound/BallBounce.BallBounce" 1.0 1.0 0.0 null null))

(fn `GetReflectionImpulse`
  (set `self.Velocity` (`self.GetVelocity` (`self.Actor`)))
  (if (`/Game/BluePrints/PhysicsBallBP.IsRightDirectionRollingMode` (`self.Actor`))
    (set `self.ReflectionImpulse` (`self.RightReflectionImpulse`))
    (else
      (set `self.ReflectionImpulse` (`self.LeftReflectionImpulse`)))))

(fn `InvertImpulse`
  (params (Impulse :type "Vector Structure"))
  (returns (Result :type "Vector Structure"))
  (return (* Impulse -1)))

(fn `ReboundFromSurface`
  (bind _result (`self.InvertImpulse` (`self.Velocity`)))
  (`PrimitiveComponent.AddImpulse` (`/Game/BluePrints/PhysicsBallBP.Ball` (`self.Actor`)) _result "None" true)
  (`PrimitiveComponent.AddImpulse` (`/Game/BluePrints/PhysicsBallBP.Ball` (`self.Actor`)) (`self.ReflectionImpulse`) "None" true))

(fn `UserConstructionScript`)