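; Hitch is a geometry Blueprint that acts on the physics ball through two trigger boxes, one to launch it and one to halt it.
; BoxBoost applies a mass-independent impulse, plays a jump sound and turns on the ball's Niagara effect.
; BoxStopDIrection zeroes the ball's linear velocity.
; Both triggers also write Damage to DamageFromCurve on the GameInstance's BallPawn, rather than through the overlapping pawn reference.
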(event `self.ReceiveBeginPlay`
  (set `self.GameInstance` (cast `/Game/BluePrints/Savings/BallGameInstance` (`GameplayStatics.GetGameInstance`) :!pure true)))

(event `self.BoxBoost.OnComponentBeginOverlap`
  (params (OverlappedComponent :type "PrimitiveComponent Object Reference") (OtherActor :type "Actor Object Reference") (OtherComp :type "PrimitiveComponent Object Reference") (OtherBodyIndex :type Integer) (bFromSweep :type Boolean) (SweepResult :type "HitResult Structure (by ref)"))
  (bind _asphysics_ball_bp (cast `/Game/BluePrints/PhysicsBallBP` OtherActor))
  (set `self.Pawn` _asphysics_ball_bp)
  (`GameplayStatics.PlaySound2D` "/Game/Sound/JumpCurveSound.JumpCurveSound" 1.0 1.0 0.0 null null)
  (set `/Game/BluePrints/Savings/BallPawn.DamageFromCurve` (`self.Damage`) (`/Game/BluePrints/Savings/BallGameInstance.BallPawn` (`self.GameInstance`)))
  (`PrimitiveComponent.AddImpulse` (`/Game/BluePrints/PhysicsBallBP.Ball` (`self.Pawn`)) (`self.Impulse`) "None" true)
  (`/Game/BluePrints/PhysicsBallBP.TurnOnNiagara` (`self.Pawn`)))

(event `self.BoxStopDIrection.OnComponentBeginOverlap`
  (params (OverlappedComponent :type "PrimitiveComponent Object Reference") (OtherActor :type "Actor Object Reference") (OtherComp :type "PrimitiveComponent Object Reference") (OtherBodyIndex :type Integer) (bFromSweep :type Boolean) (SweepResult :type "HitResult Structure (by ref)"))
  (bind _asphysics_ball_bp (cast `/Game/BluePrints/PhysicsBallBP` OtherActor))
  (set `self.Pawn` _asphysics_ball_bp)
  (set `/Game/BluePrints/Savings/BallPawn.DamageFromCurve` (`self.Damage`) (`/Game/BluePrints/Savings/BallGameInstance.BallPawn` (`self.GameInstance`)))
  (`PrimitiveComponent.SetPhysicsLinearVelocity` (`/Game/BluePrints/PhysicsBallBP.Ball` (`self.Pawn`)) (0.0 0.0 0.0) false "None"))

(fn `UserConstructionScript`)