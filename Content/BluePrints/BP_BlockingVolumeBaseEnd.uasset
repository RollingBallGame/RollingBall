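; End-of-section checkpoint volume for the physics ball, with fire particles hidden until activated.
; On first crossing it runs BaseOverlap, restores normal controls, blends the camera back to the ball, requests sunny weather and shows the fire after a delay.
; Later overlaps call ChangeHealth with the ball's max health.
; A GameInstance PrepareEnvironment event can also activate it directly, skipping the camera, control and weather resets.
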(event `self.ReceiveBeginPlay`
  (set `self.GameInstance` (cast `/Game/BluePrints/Savings/BallGameInstance` (`GameplayStatics.GetGameInstance`) :!pure true))
  (set `self.BallPawn` (cast `/Game/BluePrints/PhysicsBallBP` (`GameplayStatics.GetPlayerPawn` 0) :!pure true))
  (for _array_element (`self.K2_GetComponentsByClass` "/Script/Engine.ParticleSystemComponent")
    (`SceneComponent.SetVisibility` _array_element false false)
    (add `/Game/BluePrints/Savings/BallGameInstance.PrepareEnvironment` (`self.GameInstance`) (delegate `TurnOnFire`))))

(event `TurnOnFire`
  (`self.Base Overlap` (`self.BallPawn`))
  (set `self.IsFitrstTimeCrossed` false)
  (for _array_element (`self.K2_GetComponentsByClass` "/Script/Engine.ParticleSystemComponent")
    (`SceneComponent.SetVisibility` _array_element true false)))

(event `self.BoxTrigger.OnComponentBeginOverlap`
  (params (OverlappedComponent :type "PrimitiveComponent Object Reference") (OtherActor :type "Actor Object Reference") (OtherComp :type "PrimitiveComponent Object Reference") (OtherBodyIndex :type Integer) (bFromSweep :type Boolean) (SweepResult :type "HitResult Structure (by ref)"))
  (bind _asphysics_ball_bp (cast `/Game/BluePrints/PhysicsBallBP` OtherActor))
  (bind _output_get (set `self.BallPawn` _asphysics_ball_bp))
  (if (== (`self.IsFitrstTimeCrossed`) true)
    (`self.Base Overlap` _output_get)
    (set `self.IsFitrstTimeCrossed` false)
    (set `/Game/BluePrints/Savings/BallGameInstance.IsCameraVolumeUsing` false (cast `/Game/BluePrints/Savings/BallGameInstance` (`GameplayStatics.GetGameInstance`) :!pure true))
    (set `/Game/BluePrints/PhysicsBallBP.IsControllInverted` false (`self.BallPawn`))
    (`PlayerController.SetViewTargetWithBlend` (`GameplayStatics.GetPlayerController` 0) (`self.BallPawn`) 1.0 "VTBlend_Linear" 1.0 false)
    (`/Game/BluePrints/Savings/BallGameInstance.ChangeWeatherToSunny` (cast `/Game/BluePrints/Savings/BallGameInstance` (`GameplayStatics.GetGameInstance`) :!pure true))
    (`KismetSystemLibrary.Delay` 2.0)
    (for _array_element (`self.K2_GetComponentsByClass` "/Script/Engine.ParticleSystemComponent")
      (`SceneComponent.SetVisibility` _array_element true false))
    (else
      (`/Game/BluePrints/PhysicsBallBP.ChangeHealth` (`self.BallPawn`) (`/Game/BluePrints/Savings/BallPawn.MaxHealth` (`/Game/BluePrints/Savings/BallGameInstance.BallPawn` (`self.GameInstance`)))))))

(fn `UserConstructionScript`
  (`parent.UserConstructionScript`))